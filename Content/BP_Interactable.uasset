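; BP_Interactable is an actor that holds the basic state for an object that can be interacted with.
; At BeginPlay it binds cursor-over enter and exit handlers, which check CanBeInteracted but perform no action yet.
; Interact_Event sets the Interacting flag only when CanBeInteracted is true, while StopInteract_Event clears it unconditionally.
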(event Custom|Interact_Event
  (if (Variables|Default|GetbCanBeInteracted)
    (Variables|Default|SetbInteracting true)))

(event Custom|StopInteract_Event
  (Variables|Default|SetbInteracting false))

(event Custom|CursorOverExit_Event
  (if (Variables|Default|GetbCanBeInteracted)
    _))

(event Custom|CursorOverEnter_Event
  (if (Variables|Default|GetbCanBeInteracted)
    _))

(event EventBeginPlay
  (EventDispatchers|BindEventtoCursorOverEnter (delegate Custom|CursorOverEnter_Event))
  (EventDispatchers|BindEventtoCursorOverExit (delegate Custom|CursorOverExit_Event)))

(event Collision|EventActorBeginOverlap
  (params (OtherActor :type Actor%20Object%20Reference)))

(event EventTick
  (params (DeltaSeconds :type Float%20%28single-precision%29)))

(fn ConstructionScript)