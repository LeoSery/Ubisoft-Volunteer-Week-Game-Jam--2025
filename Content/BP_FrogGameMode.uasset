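; Game mode for a frog game that acts as the central registry and moves the view through a sequence of area cameras.
; Spawners, frogs, cameras, end ways and collectibles register with it, and each collectible receives the end way of its sequence index.
; Its Tick centrally drives the spawner and every registered frog.
; Sequence changes blend the player's view to the indexed camera, and collected mesh items are tracked without duplicates.
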(event EventBeginPlay
  (Default|Sequence|MoveCameratoSequencePosition 0 (Variables|Default|Settings|GetCameraSpeed))
  (Default|Sequence|GoNextSequence))

(event EventTick
  (params (DeltaSeconds :type Float%20%28single-precision%29))
  (Default|SpawnEntity (Variables|Default|Register|GetSpawner) DeltaSeconds)
  (for _array_element (Variables|Default|Register|GetFrogs)
    (Default|MoveFrog _array_element DeltaSeconds)))

(fn ConstructionScript)

(fn RegisterSpawner
  (params (NewSpawner :type BP%20Spawner%20Object%20Reference))
  (if (Utilities|IsValid NewSpawner)
    (Variables|Default|Register|SetSpawner NewSpawner)))

(fn RegisterFrog
  (params (NewFrog :type BP%20Frog%20Object%20Reference))
  (if (Utilities|IsValid NewFrog)
    (Utilities|Array|AddUnique (Variables|Default|Register|GetFrogs) NewFrog)))

(fn AddItemtoCollected
  (params (NewMeshItem :type Static%20Mesh%20Object%20Reference))
  (if (Utilities|IsValid NewMeshItem)
    (Utilities|Array|AddUnique (Variables|Default|Sequence|GetMeshsCollected) NewMeshItem)))

(fn UnregisterFrog
  (params (FrogToRemove :type BP%20Frog%20Object%20Reference))
  (bind _returnvalue (Utilities|Array|RemoveItem (Variables|Default|Register|GetFrogs) FrogToRemove))
  (return _returnvalue))

(fn GoNextSequence
  (if (== (Variables|Default|Settings|GetCurrentSequenceIndex) -1)
    (Default|Sequence|MoveCameratoSequencePosition (stale _result) (Variables|Default|Settings|GetCameraSpeed))
    (else
      (bind _result (Math|Integer|IncrementInt (Variables|Default|Settings|GetCurrentSequenceIndex))
        (:%20%20
          (Default|Sequence|MoveCameratoSequencePosition _result (Variables|Default|Settings|GetCameraSpeed))))))
  (Variables|Default|Settings|SetCurrentSequenceIndex _result))

(fn MoveCameratoSequencePosition
  (params (TargetSequenceID :type Integer) (CameraSpeed :type Float%20%28double-precision%29))
  (bind _areacameras (Variables|Default|Register|GetAreaCameras))
  (bind _output (Utilities|Array|Get(acopy) _areacameras TargetSequenceID))
  (if (Utilities|IsValid _output)
    (Game|Player|SetViewTargetwithBlend (Game|GetPlayerController 0) _output CameraSpeed "VTBlend_Cubic" 0.0 true)))

(fn RegisterCamera
  (params (NewCamera :type BP%20Area%20Camera%20Object%20Reference) (NewCameraIndex :type Integer))
  (if (Utilities|IsValid NewCamera)
    (Utilities|Array|SetArrayElem (Variables|Default|Register|GetAreaCameras) NewCameraIndex NewCamera true)
    (return)))

(fn RegisterEndWay
  (params (NewEndWay :type BP%20End%20Way%20Object%20Reference) (AssociatedSequenceIndex :type Integer))
  (if (Utilities|IsValid NewEndWay)
    (Utilities|Array|SetArrayElem (Variables|Default|Register|GetSequenceEndWays) AssociatedSequenceIndex NewEndWay true)
    (return)))

(fn RegisterCollectible
  (params (NewCollectible :type BP%20Collectible%20Object%20Reference) (CollectibleSequenceIndex :type Integer))
  (if (Utilities|IsValid NewCollectible)
    (Utilities|Array|AddUnique (Variables|Default|Register|GetCollectibles) NewCollectible)
    (Variables|/Game/Item/BP_Collectible.BP_Collectible_C|SetAssociatedEndWay NewCollectible (Utilities|Array|Get(acopy) (Variables|Default|Register|GetSequenceEndWays) CollectibleSequenceIndex))
    (return)))