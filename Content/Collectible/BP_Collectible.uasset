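; BP_Collectible is a pickup actor that BP_Frog collects on overlap, counting toward a linked end way.
; The construction script applies its configurable mesh and material.
; Register adds it to the GameMode's collectibles and resolves its end way by sequence index, reporting an error on failure.
; When the frog accepts the mesh, the collectible adds itself to the end way's ItemCollected and destroys itself.
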(event Collision|EventActorBeginOverlap
  (params (OtherActor :type Actor%20Object%20Reference))
  (bind _asbp_frog (Utilities|Casting|CastToBP_Frog OtherActor))
  (bind _itemwasadd (Default|AddStaticMeshItem _asbp_frog (Variables|Default|GetMeshToCollect)))
  (if _itemwasadd
    (Utilities|Array|AddUnique (Variables|/Game/BP_EndWay.BP_EndWay_C|GetItemCollected (Variables|Default|GetAssociatedEndWay)) self)
    (Actor|DestroyActor)))

(fn ConstructionScript
  (bind _itemmesh (Variables|Components|GetItemMesh))
  (Components|StaticMesh|SetStaticMesh _itemmesh (Variables|Default|GetMeshToCollect))
  (Rendering|Material|SetMaterial _itemmesh 0 (Variables|Default|GetMeshMaterial)))

(fn Register
  (params (GameMode :type BP%20Frog%20Game%20Mode%20Object%20Reference))
  (bind _sequenceendways (Variables|/Game/BP_FrogGameMode.BP_FrogGameMode_C|GetSequenceEndWays GameMode))
  (bind _associatedsequenceindex (Variables|Default|GetAssociatedSequenceIndex))
  (bind _output (Utilities|Array|Get(acopy) _sequenceendways _associatedsequenceindex))
  (if (Utilities|IsValid GameMode)
    (Utilities|Array|AddUnique (Variables|/Game/BP_FrogGameMode.BP_FrogGameMode_C|GetCollectibles GameMode) self)
    (if (Utilities|IsValid _output)
      (Variables|Default|SetAssociatedEndWay _output)
      (else
        (Default|DisplayErrorRegister GameMode (Utilities|GetDisplayName self))))
    (return)
    (else
      (Default|DisplayErrorRegister GameMode (Utilities|GetDisplayName self))
      (return))))