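; Player controller that shows the mouse cursor and lets the player hover over and click BP_Interactable actors.
; Each async physics tick runs a debug-drawn line trace from the deprojected cursor, caching the cast hit actor.
; Cursor enter and exit calls fire only when blocking-hit state changes, so moving directly between hits keeps the first target.
; Left mouse press and release start and stop interaction on the cached actor.
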(event EventBeginPlay
  (Variables|Default|SetbShowMouseCursor true))

(event EventAsyncPhysicsTick
  (params (DeltaSeconds :type Float%20%28single-precision%29) (SimSeconds :type Float%20%28single-precision%29))
  (bind (_interactable _hashit) (CallFunction|InteractableTrace))
  (if _hashit
    (if (not (Variables|Default|GetbCanInteract))
      (Variables|Default|SetbCanInteract true)
      (bind _output_get (Variables|Default|SetInteractable%20 _interactable))
      (Default|CallCursorOverEnter _output_get))
    (elif (Variables|Default|GetbCanInteract)
      (Variables|Default|SetbCanInteract false)
      (if (Utilities|IsValid (Variables|Default|GetInteractable%20))
        (Default|CallCursorOverExit (Variables|Default|GetInteractable%20))
        (Variables|Default|SetInteractable%20 0)))))

(event Input|MouseEvents|LeftMouseButton
  (params (Key :type Key%20Structure :default "None"))
  (bind _interactable_ (Variables|Default|GetInteractable%20))
  (bind _interactable__2 (Variables|Default|GetInteractable%20))
  (bind _returnvalue (Utilities|IsValid _interactable_))
  (:Pressed
    (if _returnvalue
      (Default|InteractEvent _interactable__2)
      (Variables|Default|SetbIsInteracting true)))
  (:Released
    (if (and _returnvalue (Variables|Default|GetbIsInteracting))
      (Default|StopInteractEvent _interactable__2)
      (Variables|Default|SetbIsInteracting false))))

(fn ConstructionScript)

(fn InteractableTrace
  (bind _self self)
  (bind (_worldlocation _worlddirection) (Game|Player|ConvertMouseLocationToWorldSpace _self))
  (bind _outhit (Collision|LineTraceByChannel _worldlocation (+ _worldlocation (* _worlddirection 3e+04)) "TraceTypeQuery3" false 0 "ForDuration" true "(R=1.000000,G=0.000000,B=0.000000,A=1.000000)" "(R=0.000000,G=1.000000,B=0.000000,A=1.000000)" 15.0))
  (bind _asbp_interactable (Utilities|Casting|CastToBP_Interactable (.hitactor _outhit))
    (:then
      (return _asbp_interactable (.bblockinghit _outhit)))
    (:CastFailed
      (return 0 (.bblockinghit _outhit)))))