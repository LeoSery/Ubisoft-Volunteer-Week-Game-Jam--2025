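; BP_EndWay is a trigger actor that ends a sequence in the frog game or kills the frog.
; On overlap, IsJustKill makes it purely lethal; otherwise it advances BP_FrogGameMode and destroys itself once all RequiredCollectible entries are collected, killing the frog if any are missing.
; AddCollectedItem records unique pickups for that check, and Register stores the actor in the game mode's SequenceEndWays at AssociatedSequenceID.
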(event Collision|EventActorBeginOverlap
  (params (OtherActor :type Actor%20Object%20Reference))
  (if (Variables|Default|GetIsJustKill)
    (bind _asbp_frog (Utilities|Casting|CastToBP_Frog OtherActor))
    (Default|KillFrog _asbp_frog)
    (else
      (bind _result (CallFunction|CheckEndOfSequence))
      (if _result
        (bind _asbp_frog_game_mode (Utilities|Casting|CastToBP_FrogGameMode (Game|GetGameMode)))
        (Default|GoNextSequence _asbp_frog_game_mode)
        (Actor|DestroyActor)
        (else
          (bind _asbp_frog_2 (Utilities|Casting|CastToBP_Frog OtherActor))
          (Default|KillFrog _asbp_frog_2))))))

(fn ConstructionScript)

(fn CheckEndOfSequence
  (if (== (Utilities|Array|Length (Variables|Default|GetRequiredCollectible)) 0)
    (return true)
    (else
      (LocalVariables|SetResultt true)
      (bind _array_element (Utilities|Array|ForEachLoopwithBreak (Variables|Default|GetRequiredCollectible))
        (:LoopBody
          (if (not (Utilities|Array|ContainsItem (Variables|Default|GetItemCollected) _array_element))
            (bind _output_get (LocalVariables|SetResultt (Utilities|Array|ContainsItem (Variables|Default|GetItemCollected) _array_element)))
            (return _output_get)))
        (:Completed
          (return (LocalVariables|GetResultt)))))))

(fn AddCollectedItem
  (params (NewCollectedItem :type BP%20Collectible%20Object%20Reference))
  (if (Utilities|IsValid NewCollectedItem)
    (Utilities|Array|AddUnique (Variables|Default|GetItemCollected) NewCollectedItem)
    (return)))

(fn Register
  (params (GameMode :type BP%20Frog%20Game%20Mode%20Object%20Reference))
  (if (Utilities|IsValid GameMode)
    (Utilities|Array|SetArrayElem (Variables|/Game/BP_FrogGameMode.BP_FrogGameMode_C|GetSequenceEndWays GameMode) (Variables|Default|GetAssociatedSequenceID) self true)
    (return)
    (else
      (Default|DisplayErrorRegister GameMode (Utilities|GetDisplayName self))
      (return))))