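; BP_Spawner is a placed actor that spawns BP_Frog actors at its own transform.
; On BeginPlay it registers itself with BP_FrogGameMode and marks itself active.
; SpawnEntity, while active and below the maximum frog count, spawns a frog and initializes it with this spawner as origin and the starting spline to follow.
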(event Custom|SpawnEntity
  (if (Variables|Default|GetIsActive)
    (if (< (Variables|Default|GetCurrentFrogNumber) (Variables|Default|GetMaxFrogNumber))
      (bind _returnvalue (Game|SpawnActorfromClass "/Game/Frog/BP_Frog.BP_Frog_C" (Transformation|GetActorTransform) "Undefined" "MultiplyWithRoot" 0 0))
      (Default|InitFrog _returnvalue self (Variables|Default|GetStartingSpline)))))

(event EventBeginPlay
  (bind _asbp_frog_game_mode (Utilities|Casting|CastToBP_FrogGameMode (Game|GetGameMode)))
  (Default|RegisterSpawner _asbp_frog_game_mode self)
  (Variables|Default|SetIsActive true))

(fn ConstructionScript)