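; BP_RainPoint is a rain point that registers itself with the game mode under an associated sequence index.
; Register writes the instance into the game mode's RainPoints array at that index, growing the array to fit if needed.
; When the game mode reference is invalid, it calls DisplayErrorRegister on that same invalid reference, passing its own object name.
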(fn ConstructionScript)

(fn Register
  (params (GameMode :type BP%20Frog%20Game%20Mode%20Object%20Reference))
  (if (Utilities|IsValid GameMode)
    (Utilities|Array|SetArrayElem (Variables|/Game/BP_FrogGameMode.BP_FrogGameMode_C|GetRainPoints GameMode) (Variables|Default|GetAssociatedSequenceIndex) self true)
    (return)
    (else
      (Default|DisplayErrorRegister GameMode (Utilities|GetObjectName self))
      (return))))