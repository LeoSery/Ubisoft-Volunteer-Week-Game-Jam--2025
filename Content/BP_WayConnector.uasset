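; BP_WayConnector is a junction trigger that switches an overlapping BP_Frog between a main and a variant spline path.
; It uses the variant way when ForceChangeWay is set or once its linked MiniGame reports success, otherwise the main way.
; On a switch, it passes the frog the closest point on the new spline as a start time, computed as distance over spline length.
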(event Custom|GameSucceed
  (Variables|Default|SetbShouldUseVariant true))

(event EventBeginPlay
  (if (Utilities|IsValid (Variables|Default|GetMiniGame))
    (EventDispatchers|BindEventtoSucceed (Variables|Default|GetMiniGame) (delegate Custom|GameSucceed))))

(event Collision|EventActorBeginOverlap
  (params (OtherActor :type Actor%20Object%20Reference))
  (bind _asbp_frog (Utilities|Casting|CastToBP_Frog OtherActor))
  (if (or (Variables|Default|GetbForceChangeWay) (Variables|Default|GetbShouldUseVariant))
    (CallFunction|SetFrogNewWay _asbp_frog (Variables|Default|GetVariantWay))
    (else
      (CallFunction|SetFrogNewWay _asbp_frog (Variables|Default|GetMainWay)))))

(fn ConstructionScript)

(fn SetFrogNewWay
  (params (TargetFrog :type BP%20Frog%20Object%20Reference) (NewWay :type BP%20Way%20Object%20Reference))
  (if (and (Utilities|IsValid TargetFrog) (Utilities|IsValid NewWay))
    (if (!= (Variables|/Game/Frog/BP_Frog.BP_Frog_C|GetSplineToFollow TargetFrog) NewWay)
      (bind _closesttimeonspline (CallFunction|GetClosestTimeonSpline NewWay (Transformation|GetActorLocation TargetFrog)))
      (Default|SetNewSplinetoFollow TargetFrog NewWay _closesttimeonspline)
      (return)
      (else
        (return)))))

(fn GetClosestTimeonSpline
  (params (TargetSpline :type BP%20Way%20Object%20Reference) (WorldLocation :type Vector))
  (bind _spline (Variables|/Game/BP_Way.BP_Way_C|GetSpline TargetSpline))
  (return (/ (Class|SplineComponent|GetDistanceAlongSplineatLocation _spline (Spline|FindLocationClosesttoWorldLocation _spline WorldLocation "World") "World") (Spline|GetSplineLength _spline))))